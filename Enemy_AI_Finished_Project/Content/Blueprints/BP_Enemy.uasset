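; Enemy Blueprint that randomly patrols, chases the third-person player on detection and plays a mutant melee attack montage.
; Detection overlaps switch between patrol and a looping timer that refreshes the AI MoveTo toward the player.
; On arrival, an attack-range overlap flag gates the montage, and chasing resumes afterward if the player remains detected.
; A damage collision, gated by CanDealDamage, only prints a message; nothing here sets that flag.
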(event OnComponentBeginOverlap(PlayerAttackCollisionDetection)
  (params (OverlappedComponent :type Primitive%20Component%20Object%20Reference) (OtherActor :type Actor%20Object%20Reference) (OtherComp :type Primitive%20Component%20Object%20Reference) (OtherBodyIndex :type Integer) (bFromSweep :type Boolean) (SweepResult :type Hit%20Result%20Structure%20%28by%20ref%29))
  (Utilities|Casting|CastToThirdPersonCharacter OtherActor)
  (Variables|Default|SetCan%20Attack%20Player true))

(event OnComponentEndOverlap(PlayerAttackCollisionDetection)
  (params (OverlappedComponent :type Primitive%20Component%20Object%20Reference) (OtherActor :type Actor%20Object%20Reference) (OtherComp :type Primitive%20Component%20Object%20Reference) (OtherBodyIndex :type Integer))
  (Utilities|Casting|CastToThirdPersonCharacter OtherActor)
  (Variables|Default|SetCan%20Attack%20Player false))

(event OnComponentBeginOverlap(DamageCollision)
  (params (OverlappedComponent :type Primitive%20Component%20Object%20Reference) (OtherActor :type Actor%20Object%20Reference) (OtherComp :type Primitive%20Component%20Object%20Reference) (OtherBodyIndex :type Integer) (bFromSweep :type Boolean) (SweepResult :type Hit%20Result%20Structure%20%28by%20ref%29))
  (Utilities|Casting|CastToThirdPersonCharacter OtherActor)
  (if (Variables|Default|GetCan%20Deal%20Damage)
    (Development|PrintString "Player Damaged")))

(event OnComponentBeginOverlap(PlayerCollisionDetection)
  (params (OverlappedComponent :type Primitive%20Component%20Object%20Reference) (OtherActor :type Actor%20Object%20Reference) (OtherComp :type Primitive%20Component%20Object%20Reference) (OtherBodyIndex :type Integer) (bFromSweep :type Boolean) (SweepResult :type Hit%20Result%20Structure%20%28by%20ref%29))
  (bind _asthird_person_character (Utilities|Casting|CastToThirdPersonCharacter OtherActor))
  (Variables|Default|SetPlayer%20REF _asthird_person_character)
  (Variables|Default|SetPlayer%20Detected true)
  (CallFunction|SeekPlayer))

(event OnComponentEndOverlap(PlayerCollisionDetection)
  (params (OverlappedComponent :type Primitive%20Component%20Object%20Reference) (OtherActor :type Actor%20Object%20Reference) (OtherComp :type Primitive%20Component%20Object%20Reference) (OtherBodyIndex :type Integer))
  (Utilities|Casting|CastToThirdPersonCharacter OtherActor)
  (Variables|Default|SetPlayer%20Detected false)
  (CallFunction|StopSeekingPlayer)
  (CallFunction|RandomPatrol))

(event Custom|Random%20Patrol
  (AI|AIMoveTo self (.RandomLocation (AI|Navigation|GetRandomReachablePointinRadius (Transformation|GetActorLocation) 2.5e+03 0 0)) 0 5.0 false
    (:OnSuccess
      (CallFunction|RandomPatrol))))

(event Custom|Move%20To%20Player
  (AI|AIMoveTo self (Transformation|GetActorLocation (Variables|Default|GetPlayer%20REF)) 0 1.5e+02 false
    (:OnSuccess
      (if (Variables|Default|GetCan%20Attack%20Player)
        (CallFunction|StopSeekingPlayer)
        (Animation|Montage|PlayMontage (Variables|Character|GetMesh) "/Game/Enemy_Model/Mutant_Attack_Montage.Mutant_Attack_Montage"
          (:OnCompleted
            (if (Variables|Default|GetPlayer%20Detected)
              (CallFunction|SeekPlayer))))
        (else
          (CallFunction|SeekPlayer))))))

(event Custom|Seek%20Player
  (CallFunction|MovetoPlayer)
  (Utilities|Time|SetTimerbyFunctionName 0 "Seek Player" 0.25 true))

(event Custom|Stop%20Seeking%20Player
  (Utilities|Time|ClearTimerbyFunctionName 0 "Seek Player"))

(event EventBeginPlay
  (CallFunction|RandomPatrol))

(fn ConstructionScript)